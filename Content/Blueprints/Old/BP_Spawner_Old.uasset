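; BP_Spawner_Old is a bullet spawner actor in the Old folder, with its firing logic disconnected.
; BeginPlay starts looping timers for an empty FireBullet event and for ChangeDirection, which cycles Direction through four entries of a Directions array.
; Tick caches the actor's location as SpawnLocation.
; The randomly rotated bullet spawn and other leftover nodes never run, so nothing is spawned.
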(event `self.ReceiveBeginPlay`
  (`KismetSystemLibrary.K2_SetTimerDelegate` (delegate `FireBullet`) (`self.FireRate`) true)
  (`KismetSystemLibrary.K2_SetTimerDelegate` (delegate `ChangeDirection`) 3.0 true))

(event `FireBullet`)

(event `ChangeDirection`
  (set `self.Direction` (`|GetArrayItem` (`self.Directions`) (`self.CurrentIndex`)))
  (if (== (`self.CurrentIndex`) 3)
    (set `self.CurrentIndex` 0)
    (else
      (set `self.CurrentIndex` (+ (`self.CurrentIndex`) 1)))))

(event `self.ReceiveTick`
  (params (DeltaSeconds :type "Float (single-precision)"))
  (set `self.SpawnLocation` (`self.K2_GetActorLocation`)))

(fn `UserConstructionScript`)