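; BP_Meteorite is a destructible meteorite actor that loses health when hit by bullets.
; On overlap, it casts the other actor to BP_Bullet_Old or BP_Bullet_Child_Old, destroys the bullet, decrements CurrentHealth and prints debug text.
; Tick polls CurrentHealth and destroys the meteorite at zero or below.
; BeginPlay starts a looping FireRate timer for FireBullet, which is empty, and unconnected location nodes never run.
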(event `self.ReceiveBeginPlay`
  (`KismetSystemLibrary.K2_SetTimerDelegate` (delegate `FireBullet`) (`self.FireRate`) true))

(event `FireBullet`)

(event `self.ReceiveTick`
  (params (DeltaSeconds :type "Float (single-precision)"))
  (if (<= (`self.CurrentHealth`) 0.0)
    (`self.K2_DestroyActor`)))

(event `self.ReceiveActorBeginOverlap`
  (params (OtherActor :type "Actor Object Reference"))
  (`KismetSystemLibrary.PrintString` "hi")
  (bind _asbp_bullet (cast `/Game/Blueprints/BP_Bullet_Old` OtherActor)
    (:`then`
      (`self.K2_DestroyActor` _asbp_bullet :!label _label)
      (`self.K2_DestroyActor` (stale _asbp_bullet_child))
      (set `self.CurrentHealth` (- (`self.CurrentHealth`) 1.0))
      (`KismetSystemLibrary.PrintString` "meteorite took damage"))
    (:`CastFailed`
      (bind _asbp_bullet_child (cast `/Game/Blueprints/BP_Bullet_Child_Old` OtherActor))
      (if (`KismetSystemLibrary.IsValid` _asbp_bullet_child)
        (goto _label)))))

(fn `UserConstructionScript`)