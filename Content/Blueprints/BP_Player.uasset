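; Player UFO pawn for a bullet-hell shooter, with Enhanced Input flight, look, shooting and an energy-costing Timeline dash.
; Tick queries BP_BulletManager at two radii: hits reduce health and return the bullet, while grazes pulse WB_Bar and add energy.
; Energy drains steadily; higher levels shorten the looping fire timer's interval and, near the top, turn single shots into a three-way spread.
; Movement input drives interpolated tilt on the ship and camera.
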(event `EnhancedInput|/Game/Input/IA_Fly`
  (params (ActionValue :type "Float (double-precision)") (ElapsedSeconds :type "Float (double-precision)") (TriggeredSeconds :type "Float (double-precision)") (InputAction :type "InputAction Object Reference" :default "/Game/Input/IA_Fly.IA_Fly"))
  (:`Triggered`
    (`self.AddMovementInput` (`KismetMathLibrary.MakeVector` 0.0 0.0 ActionValue) (`self.MovementSpeed`))))

(event `EnhancedInput|/Game/Input/IA_Dash`
  (params (ActionValue :type Boolean) (ElapsedSeconds :type "Float (double-precision)") (TriggeredSeconds :type "Float (double-precision)") (InputAction :type "InputAction Object Reference" :default "/Game/Input/IA_Dash.IA_Dash"))
  (bind _returnvalue (`PawnMovementComponent.GetLastInputVector` (`self.FloatingPawnMovement`)))
  (:`Started`
    (if (>= (`self.CurrentEnergy`) 10.0)
      (set `self.CurrentEnergy` (`KismetMathLibrary.FMax` (- (`self.CurrentEnergy`) 10.0)))
      (bind (_direction _newtrack_0) (`Timeline|Timeline` :!via `PlayFromStart`)
        (:`Update`
          (if (== _returnvalue (0.0 0.0 0.0) :`ErrorTolerance` 0.001)
            (bind _returnvalue_2 (* (`self.GetActorForwardVector`) (`KismetMathLibrary.Conv_DoubleToVector` (* _newtrack_0 1000.0))))
            (`self.K2_AddActorWorldOffset` _returnvalue_2 true)
            (`KismetSystemLibrary.PrintString` (`KismetStringLibrary.Conv_VectorToString` _returnvalue_2))
            (else
              (`self.K2_AddActorWorldOffset` (* _returnvalue _newtrack_0) true))))))))

(event `self.ReceiveBeginPlay`
  (bind _returnvalue (`GameplayStatics.GetPlayerCameraManager` 0))
  (`EnhancedInputSubsystemInterface.AddMappingContext` (pcsubsystem `EnhancedInputLocalPlayerSubsystem` (`GameplayStatics.GetPlayerController` 0)) "/Game/Input/IMC_FreeCam.IMC_FreeCam" 0 (struct))
  (set `PlayerCameraManager.ViewPitchMax` 89.42 _returnvalue)
  (set `PlayerCameraManager.ViewPitchMin` -89.42 _returnvalue))

(event `EnhancedInput|/Game/Input/IA_Move`
  (params (ActionValue :type "Vector2D Structure") (ElapsedSeconds :type "Float (double-precision)") (TriggeredSeconds :type "Float (double-precision)") (InputAction :type "InputAction Object Reference" :default "/Game/Input/IA_Move.IA_Move"))
  (bind _movementspeed (`self.MovementSpeed`))
  (:`Triggered`
    (`self.AddMovementInput` (`KismetMathLibrary.Normal` (`KismetMathLibrary.MakeVector` (.x (`self.GetActorRightVector`)) (.y (`self.GetActorRightVector`)))) (* ActionValue_X _movementspeed))
    (`self.AddMovementInput` (`KismetMathLibrary.Normal` (`KismetMathLibrary.MakeVector` (.x (`self.GetActorForwardVector`)) (.y (`self.GetActorForwardVector`)))) (* ActionValue_Y _movementspeed))
    (set `self.Action Value X` ActionValue_X :!label _label)
    (set `self.Action Value Y` (* ActionValue_Y -1.0)))
  (:`Completed`
    (goto _label)))

(event `EnhancedInput|/Game/Input/IA_Look`
  (params (ActionValue :type "Vector2D Structure") (ElapsedSeconds :type "Float (double-precision)") (TriggeredSeconds :type "Float (double-precision)") (InputAction :type "InputAction Object Reference" :default "/Game/Input/IA_Look.IA_Look"))
  (:`Triggered`
    (`self.AddControllerYawInput` ActionValue_X)
    (`self.AddControllerPitchInput` (* -1.0 ActionValue_Y))))

(event `self.ReceiveTick`
  (params (DeltaSeconds :type "Float (single-precision)"))
  (bind _currentenergy (`self.CurrentEnergy`))
  (`|ExecutionSequence`
    (:`then_0`
      (bind _returnvalue (`GameplayStatics.GetActorOfClass` "/Game/Blueprints/BP_BulletManager.BP_BulletManager_C"))
      (`|ExecutionSequence`
        (:`then_0`
          (bind _outbullets (`CPP_BulletManager.QueryBulletsAt` _returnvalue (`self.K2_GetActorLocation` self) 40.0))
          (if (> (`KismetArrayLibrary.Array_Length` _outbullets) 0)
            (`CPP_BulletManager.ReturnBullet` (`CPP_BulletManager.Get`) (`|GetArrayItem` _outbullets))
            (`KismetSystemLibrary.PrintText` (`KismetTextLibrary.Conv_DoubleToText` (stale _output_get) "HalfToEven"))
            (bind _output_get (set `self.CurrentHealth` (- (`self.CurrentHealth`) 1.0)))))
        (:`then_1`
          (if (> (`KismetArrayLibrary.Array_Length` (`CPP_BulletManager.QueryBulletsAt` _returnvalue (`self.K2_GetActorLocation`) 160.0)) 0)
            (`KismetSystemLibrary.PrintString` "graze")
            (`|ExecutionSequence`
              (:`then_0`
                (bind _foundwidgets (`WidgetBlueprintLibrary.GetAllWidgetsOfClass` "/Game/Blueprints/WB_Bar.WB_Bar_C"))
                (bind _output (`|GetArrayItem` _foundwidgets))
                (`UserWidget.PlayAnimation` _output (`/Game/Blueprints/WB_Bar.graze_pulse` _output) 0.0 1 "Forward" 1.0 true))
              (:`then_1`
                (if (<= _currentenergy (`self.MaxEnergy`))
                  (set `self.CurrentEnergy` (+ _currentenergy 0.75)))))))
        (:`then_2`
          (bind _output_get_2 (set `self.CurrentEnergy` (`KismetMathLibrary.FMax` 0.0 (- (`self.CurrentEnergy`) 0.05))))
          (if (<= _output_get_2 50.0)
            (set `self.FireInterval` 0.25)
            (else
              (set `self.FireInterval` 0.1))))))
    (:`then_1`
      (if (not (== (`self.FireInterval`) (`self.OldFireInterval`)))
        (set `self.OldFireInterval` (`self.FireInterval`))
        (`KismetSystemLibrary.K2_ClearAndInvalidateTimerHandle` (`self.FireTimer`))
        (if (stale `EnhancedInput|/Game/Input/IA_Shoot` ActionValue)
          (bind _returnvalue_2 (`KismetSystemLibrary.K2_SetTimerDelegate` (delegate `Fire1`) (`self.FireInterval`) true :!label _label_2))
          (set `self.FireTimer` _returnvalue_2))))
    (:`then_2`
      (bind _output_get_3 (set `self.TargetRoll` (* (`self.Action Value X`) 15.0)))
      (bind _output_get_4 (set `self.CurrentRollAngle` (`KismetMathLibrary.FInterpTo` (`self.CurrentRollAngle`) _output_get_3 (`GameplayStatics.GetWorldDeltaSeconds`) 2.0)))
      (bind _output_get_5 (set `self.TargetPitch` (* (`self.Action Value Y`) 10.0)))
      (bind _output_get_6 (set `self.CurrentPitchAngle` (`KismetMathLibrary.FInterpTo` (`self.CurrentPitchAngle`) _output_get_5 (`GameplayStatics.GetWorldDeltaSeconds`) 2.0)))
      (`SceneComponent.K2_SetRelativeRotation` (`self.ufo`) (`KismetMathLibrary.MakeRotator` _output_get_4 _output_get_6) false false)
      (bind _output_get_7 (set `self.CameraRollAngle` (`KismetMathLibrary.FInterpTo` (`self.CameraRollAngle`) (* (`self.TargetRoll`) 0.5) (`GameplayStatics.GetWorldDeltaSeconds`) 2.25)))
      (bind _output_get_8 (set `self.CameraPitchAngle` (`KismetMathLibrary.FInterpTo` (`self.CameraPitchAngle`) (* (`self.TargetPitch`) 0.25) (`GameplayStatics.GetWorldDeltaSeconds`) 2.25)))
      (`SceneComponent.K2_SetRelativeRotation` (`self.Camera`) (`KismetMathLibrary.MakeRotator` _output_get_7 _output_get_8) false false))))

(event `EnhancedInput|/Game/Input/IA_Shoot`
  (params (ActionValue :type Boolean) (ElapsedSeconds :type "Float (double-precision)") (TriggeredSeconds :type "Float (double-precision)") (InputAction :type "InputAction Object Reference" :default "/Game/Input/IA_Shoot.IA_Shoot"))
  (:`Started`
    (goto _label_2))
  (:`Completed`
    (`KismetSystemLibrary.K2_SetTimerDelegate` (delegate `Fire1`))))

(event `Fire1`
  (bind _returnvalue (`self.K2_GetActorLocation`))
  (bind _returnvalue_2 (`self.GetActorForwardVector`))
  (bind _returnvalue_3 (`self.GetActorUpVector`))
  (if (>= (`self.CurrentEnergy`) 85.0)
    (`|SpawnActorFromClass` "/Game/Blueprints/BP_Bullet_Player.BP_Bullet_Player_C" (`KismetMathLibrary.MakeTransform` _returnvalue (`KismetMathLibrary.Conv_VectorToRotator` _returnvalue_2)) "Undefined" "MultiplyWithRoot" null null)
    (`|SpawnActorFromClass` "/Game/Blueprints/BP_Bullet_Player.BP_Bullet_Player_C" (`KismetMathLibrary.MakeTransform` _returnvalue (`KismetMathLibrary.Conv_VectorToRotator` (`KismetMathLibrary.RotateAngleAxis` _returnvalue_2 -5.0 _returnvalue_3))) "Undefined" "MultiplyWithRoot" null null)
    (`|SpawnActorFromClass` "/Game/Blueprints/BP_Bullet_Player.BP_Bullet_Player_C" (`KismetMathLibrary.MakeTransform` _returnvalue (`KismetMathLibrary.Conv_VectorToRotator` (`KismetMathLibrary.RotateAngleAxis` _returnvalue_2 5.0 _returnvalue_3))) "Undefined" "MultiplyWithRoot" null null)
    (else
      (bind _returnvalue_4 (`|SpawnActorFromClass` "/Game/Blueprints/BP_Bullet_Player.BP_Bullet_Player_C" (`KismetMathLibrary.MakeTransform` (`self.K2_GetActorLocation`) (`KismetMathLibrary.Conv_VectorToRotator` (`self.GetActorForwardVector`))) "Undefined" "MultiplyWithRoot" null null)))))

(fn `UserConstructionScript`)