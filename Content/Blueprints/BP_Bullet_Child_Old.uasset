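; BP_Bullet_Child_Old is a child bullet Blueprint that destroys spawners it hits and leaves the player's health unchanged.
; Box overlap casts the other actor to BP_Player, writing CurrentHealth back to itself, otherwise to BP_Spawner_Old, which it destroys.
; BeginPlay runs the parent logic, then tints the Niagara effect an overbright HDR blue through its BulletColor parameter.
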(event `self.Box.OnComponentBeginOverlap`
  (params (OverlappedComponent :type "PrimitiveComponent Object Reference") (OtherActor :type "Actor Object Reference") (OtherComp :type "PrimitiveComponent Object Reference") (OtherBodyIndex :type Integer) (bFromSweep :type Boolean) (SweepResult :type "HitResult Structure (by ref)"))
  (bind _asbp_player (cast `/Game/Blueprints/BP_Player` OtherActor)
    (:`then`
      (set `/Game/Blueprints/BP_Player.CurrentHealth` (`/Game/Blueprints/BP_Player.CurrentHealth` _asbp_player) _asbp_player))
    (:`CastFailed`
      (bind _asbp_spawner_old (cast `/Game/Blueprints/Old/BP_Spawner_Old` OtherActor))
      (`self.K2_DestroyActor` _asbp_spawner_old))))

(event `self.ReceiveActorBeginOverlap`
  (params (OtherActor :type "Actor Object Reference")))

(event `self.ReceiveBeginPlay`
  (`parent.ReceiveBeginPlay`)
  (`FXSystemComponent.SetColorParameter` (`self.Niagara`) "BulletColor" (make `LinearColor` 0.353 41.955 268.11 1.0)))

(fn `UserConstructionScript`
  (`parent.UserConstructionScript`))